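; BP_Cheese is a cheese objective actor that announces when the player has retrieved it.
; On BeginPlay it plays a spotlight ambience cue at very low pitch, positioned by the root component's relative location.
; A Box overlap with BP_ThirdPersonCharacterCustom only prints the success message, leaving the cheese in place.
; An unconnected leftover chain would print a random elemental type but never runs.
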(event OnComponentBeginOverlap(Box)
  (params (OverlappedComponent :type Primitive%20Component%20Object%20Reference) (OtherActor :type Actor%20Object%20Reference) (OtherComp :type Primitive%20Component%20Object%20Reference) (OtherBodyIndex :type Integer) (bFromSweep :type Boolean) (SweepResult :type Hit%20Result%20Structure%20%28by%20ref%29))
  (Utilities|Casting|CastToBP_ThirdPersonCharacterCustom OtherActor)
  (Development|PrintString "You have successfully retrieved your precious piece of cheese!"))

(event EventBeginPlay
  (Audio|PlaySoundatLocation "/Game/Audio/Spotlight_Ambience_Cue.Spotlight_Ambience_Cue" (Variables|/Script/Engine.SceneComponent|GetRelativeLocation (Variables|Default|GetDefaultSceneRoot)) "0, 0, 0" 1.0 0.005 0.0 0 0 0 0))

(fn ConstructionScript)